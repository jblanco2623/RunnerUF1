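; Spawner actor that repeatedly creates Obstacle_1 actors at its own root transform while the game is running.
; BeginPlay caches the CustomMode game mode, and Tick checks its GameStarted flag before each spawn.
; A randomized Delay inside Tick paces spawning to every few seconds, and each obstacle gets a fixed life span so it cleans itself up.
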(event `self.ReceiveBeginPlay`
  (bind _ascustom_mode (cast `/Game/CustomMode` (`GameplayStatics.GetGameMode`)))
  (set `self.GameMode` _ascustom_mode))

(event `self.ReceiveTick`
  (params (DeltaSeconds :type "Float (single-precision)"))
  (if (`/Game/CustomMode.GameStarted` (`self.GameMode`))
    (`KismetSystemLibrary.Delay` (`KismetMathLibrary.RandomFloatInRange` 1.0 3.0))
    (bind _returnvalue (`|SpawnActorFromClass` "/Game/Characters/Obstacle_1.Obstacle_1_C" (`SceneComponent.K2_GetComponentToWorld` (`self.DefaultSceneRoot`)) "Undefined" "OverrideRootScale" null null))
    (`self.SetLifeSpan` _returnvalue 50.0)))

(fn `UserConstructionScript`)